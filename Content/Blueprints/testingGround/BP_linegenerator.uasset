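; Testing actor that draws a line graph through points using Niagara beams.
; The construction script builds the points from hardcoded heights at even X spacing, and BeginPlay prints and debug-draws each, calling DrawOptimizedLine on every iteration.
; That function adds one Niagara component and writes all segments to indexed BS_/BE_ parameters, with modulo wrapping back to the first point.
; Unused helpers instead spawn one beam per segment, skipping equal-height pairs.
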(event `self.ReceiveBeginPlay`
  (for _array_element (`self.Location`)
    (`KismetSystemLibrary.PrintString` (`KismetStringLibrary.Conv_VectorToString` _array_element))
    (`KismetSystemLibrary.DrawDebugPoint` _array_element 10.0 (struct) 3.0)
    (`self.DrawOptimizedLine` (`self.Location`))))

(fn `DrawLine_test`
  (params (points :type "Array of Vector Structure"))
  (locals (pt1 :type "Vector Structure") (pt2 :type "Vector Structure") (NGReference :type "NiagaraComponent Object Reference"))
  (bind _returnvalue (`KismetArrayLibrary.Array_Length` points))
  (bind _location (`self.Location`))
  (bind _returnvalue_2 (`AddComponent|NODE_AddNiagaraComponent-2`))
  (set `local.NGReference` _returnvalue_2)
  (for _index (range (+ (+ _returnvalue 1) 1))
    (set `local.pt1` (`|GetArrayItem` _location (mod _index _returnvalue)))
    (set `local.pt2` (`|GetArrayItem` _location (mod (+ _index 1) _returnvalue)))
    (if (not (== (.z (`local.pt1`)) (.z (`local.pt2`))))
      (bind _returnvalue_3 (`AddComponent|NODE_AddNiagaraComponent-0`))
      (`FXSystemComponent.SetVectorParameter` _returnvalue_3 "BeamStart" (`local.pt1`))
      (`FXSystemComponent.SetVectorParameter` _returnvalue_3 "BeamEnd" (`local.pt2`)))))

(fn `DrawNGLine`
  (params (Start :type "Vector Structure") (End :type "Vector Structure"))
  (returns (BGref :type "NiagaraComponent Object Reference"))
  ;[1 1 1] don't draw line if both points are zero
  (if (not (== (.z Start) (.z End)))
    (bind _returnvalue (`AddComponent|NODE_AddNiagaraComponent-1`))
    ;[1 1 1] set the start and end of the Niagara system
    (`self.UpdateLineStartEnd` _returnvalue Start End)
    (return _returnvalue)))

(fn `DrawOptimizedLine`
  (params (Points :type "Array of Vector Structure"))
  (locals (Pt1 :type "Vector Structure") (Pt2 :type "Vector Structure") (NGReference :type "NiagaraComponent Object Reference"))
  (bind _returnvalue (`KismetArrayLibrary.Array_Length` Points))
  (bind _points (`local.Points`))
  (bind _returnvalue_2 (`AddComponent|NODE_AddNiagaraComponent-3`))
  (set `local.NGReference` _returnvalue_2)
  (for _index (range (+ _returnvalue 1))
    (bind _returnvalue_3 (mod _index _returnvalue))
    (set `local.Pt1` (`|GetArrayItem` _points _returnvalue_3))
    (set `local.Pt2` (`|GetArrayItem` _points (mod (+ _index 1) _returnvalue)))
    (bind _returnvalue_4 (`KismetStringLibrary.Conv_IntToString` _returnvalue_3))
    (`NiagaraComponent.SetVariableVec3` (`local.NGReference`) (`KismetStringLibrary.Conv_StringToName` (`KismetStringLibrary.Concat_StrStr` "BS_" _returnvalue_4)) (`local.Pt1`))
    (`NiagaraComponent.SetVariableVec3` (`local.NGReference`) (`KismetStringLibrary.Conv_StringToName` (`KismetStringLibrary.Concat_StrStr` "BE_" _returnvalue_4)) (`local.Pt2`))))

(fn `UpdateLineStartEnd`
  (params (NGLine :type "NiagaraComponent Object Reference") (Start :type "Vector Structure") (End :type "Vector Structure"))
  (`FXSystemComponent.SetVectorParameter` NGLine "BeamStart" Start)
  (`FXSystemComponent.SetVectorParameter` NGLine "BeamEnd" End))

(fn `UserConstructionScript`
  (bind _output_get (set `self.Z_axis` (`|MakeArray` 1.0 2.0 0.0 0.0 3.0 5.0 0.0 :!type "Float (single-precision)")))
  (for (_array_element _array_index) _output_get
    (`KismetArrayLibrary.Array_Add` (`self.Location`) (`KismetMathLibrary.MakeVector` (* _array_index 50.0) 0.0 (+ (* _array_element 100.0) 20.0)))))