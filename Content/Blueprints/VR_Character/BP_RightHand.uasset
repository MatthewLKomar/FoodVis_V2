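; Right-hand Blueprint for the VR character, handling a pointing gesture for widget interaction.
; Point shows the WidgetInteraction debug display only while the top key and grip flags are both set.
; PointPress also requires the trigger flag but leads to an empty sequence; its left-mouse press and line-trace hit print are disconnected and never run.
; The event graph holds only disabled placeholder events.
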(fn `Point`
  (bind _widgetinteraction (`self.WidgetInteraction`))
  (if (and (`self.isTopKey`) (`self.IsGrip`))
    (set `WidgetInteractionComponent.bShowDebug` true _widgetinteraction)
    (else
      (set `WidgetInteractionComponent.bShowDebug` false _widgetinteraction))))

(fn `Point_Press`
  (if (and (`self.isTopKey`) (`self.IsGrip`) (`self.IsTrigger`))
    (`|ExecutionSequence`)))

(fn `UserConstructionScript`
  (`parent.UserConstructionScript`))