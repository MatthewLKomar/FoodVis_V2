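; Generator actor that visualizes food flavor data as a ring of nine flavor-group axes with debug lines linking each food's points.
; Construction loads flavor DataTables, computes circular axis locations and caches food IDs from DT_FoodID.
; BeginPlay spawns a BP_Axis per group, then gathers each food's coordinates from those axes' PointCoords maps.
; ConnectPoints draws temporary lines from each point to that food's first point; PrintPoints is unwired debug output.
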(event `self.ReceiveBeginPlay`
  (`self.SpawnAxis`)
  (`self.FindPoints`)
  (`self.ConnectPoints`))

(fn `ConnectPoints`
  (for _array_element (`self.Points`)
    (bind _returnvalue (`KismetArrayLibrary.Array_Length` (break `/Game/FlavorData/FPoints` _array_element)))
    (bind _returnvalue_2 (+ _returnvalue 1))
    (for _index (range (+ _returnvalue_2 1))
      (bind _output_vector (break `/Game/FlavorData/FPoint` (`|GetArrayItem` (break `/Game/FlavorData/FPoints` _array_element) (mod _index _returnvalue))))
      (bind _output_vector_2 (break `/Game/FlavorData/FPoint` (`|GetArrayItem` (break `/Game/FlavorData/FPoints` _array_element) (mod 0 _returnvalue_2))))
      (`KismetSystemLibrary.DrawDebugLine` _output_vector _output_vector_2 (struct :`G` 0.911458 :`B` 0.885485 :`A` 1.0) 20.0))))

(fn `FindPoints`
  (locals (PointsSeenDuringLoop :type "/Game/FlavorData/FPoints Structure"))
  (bind _pointsseenduringloop_point (break `/Game/FlavorData/FPoints` (`local.PointsSeenDuringLoop`)))
  (for (_array_element _array_index) (`self.Food_ID_Metadata`)
    (`KismetArrayLibrary.Array_Set` (`self.AxisPoints`) _array_index _array_element true)
    (for _array_element_2 (`self.AxisRefs`)
      (bind (_value _returnvalue) (`BlueprintMapLibrary.Map_Find` (`/Game/Blueprints/BP_Axis.PointCoords` _array_element_2) _array_element))
      (if _returnvalue
        (`KismetArrayLibrary.Array_Add` _pointsseenduringloop_point _value)))
    (`KismetArrayLibrary.Array_Add` (`self.Points`) (`local.PointsSeenDuringLoop`))
    (set `local.PointsSeenDuringLoop` (struct))))

(fn `GetAxisSpawnData`
  (bind (_returnvalue_x _returnvalue_y _returnvalue_z) (`KismetMathLibrary.BreakVector` (`self.K2_GetActorLocation`)))
  (for _index (range (+ (`self.MaxAxes`) 1))
    (bind _returnvalue (* _index (/ 360.0 (`KismetMathLibrary.Conv_IntToDouble` (`self.MaxAxes`)))))
    (`KismetArrayLibrary.Array_Set` (`self.AxisLocations`) _index (make `/Game/FlavorData/FAxisEntries` (`KismetMathLibrary.MakeVector` (+ _returnvalue_x (* (`self.Radius`) (`KismetMathLibrary.DegSin` _returnvalue))) (+ _returnvalue_y (* (`self.Radius`) (`KismetMathLibrary.DegCos` _returnvalue))) _returnvalue_z) (`|GetArrayItem` (`self.FlavorGroupName`) _index) (`|GetArrayItem` (`self.FlavorGroupNames`) _index)) true)))

(fn `InitFoodIDMetaData`
  (bind _outrownames (`DataTableFunctionLibrary.GetDataTableRowNames` "/Game/FlavorData/DT_FoodID.DT_FoodID"))
  (for (_array_element _array_index) _outrownames
    (bind _returnvalue (`|GetDataTableRow` "/Game/FlavorData/DT_FoodID.DT_FoodID" _array_element)
      (:`then`
        (`KismetArrayLibrary.Array_Set` (`self.Food_ID_Metadata`) _array_index (break `/Game/FlavorData/FFoodId` _returnvalue) true)))))

(fn `LoadAxisData`
  (set `self.FlavorGroupNames` (`|MakeArray` "sweet" "floral" "fruity" "green" "animal" "smoky" "wine_like" "chemical" "milky" :!type "Name"))
  (set `self.FlavorGroupName` (`|MakeArray` "/Game/FlavorData/DT_perflavor/DT_F_SWEET.DT_F_SWEET" "/Game/FlavorData/DT_perflavor/DT_F_FLORAL.DT_F_FLORAL" "/Game/FlavorData/DT_perflavor/DT_F_FRUITY.DT_F_FRUITY" "/Game/FlavorData/DT_perflavor/DT_F_GREEN.DT_F_GREEN" "/Game/FlavorData/DT_perflavor/DT_F_ANIMAL.DT_F_ANIMAL" "/Game/FlavorData/DT_perflavor/DT_F_SMOKY.DT_F_SMOKY" "/Game/FlavorData/DT_perflavor/DT_F_WINELIKE.DT_F_WINELIKE" "/Game/FlavorData/DT_perflavor/DT_F_CHEMICAL.DT_F_CHEMICAL" "/Game/FlavorData/DT_perflavor/DT_F_MILKY.DT_F_MILKY" :!type "DataTable Object Reference")))

(fn `PrintPoints`
  (locals (`Point Locations` :type String) (NumOfPoints :type Integer))
  (`KismetSystemLibrary.PrintString` (`KismetStringLibrary.Concat_StrStr` "Length of Unique Food_IDs stored: " (`KismetStringLibrary.Conv_IntToString` (`KismetArrayLibrary.Array_Length` (`self.Points`))) " Length of Unique Food_IDs:" (`KismetStringLibrary.Conv_IntToString` (`KismetArrayLibrary.Array_Length` (`self.AxisPoints`)))))
  (for (_array_element _array_index) (`self.Points`)
    (`KismetSystemLibrary.PrintString` (`KismetStringLibrary.Concat_StrStr` "Food_ID: " (`KismetStringLibrary.Conv_IntToString` (`|GetArrayItem` (`self.AxisPoints`) _array_index)) "Corresponds to: " (`KismetStringLibrary.Conv_IntToString` (`KismetArrayLibrary.Array_Length` (break `/Game/FlavorData/FPoints` _array_element))) " Points"))))

(fn `SpawnAxis`
  (for (_array_element _array_index) (`self.AxisLocations`)
    (bind (_location _data _name) (break `/Game/FlavorData/FAxisEntries` _array_element))
    (bind _returnvalue (`|SpawnActorFromClass` "/Game/Blueprints/BP_Axis.BP_Axis_C" (`KismetMathLibrary.MakeTransform` _location) "AlwaysSpawn" "OverrideRootScale" null (`KismetTextLibrary.Conv_NameToText` _name) _data null))
    (`KismetArrayLibrary.Array_Set` (`self.AxisRefs`) _array_index _returnvalue true)))

(fn `UserConstructionScript`
  (locals (FlavorGroupNames :type "Array of Name") (FlavorGroupName :type "Array of DataTable Object Reference"))
  (`self.LoadAxisData`)
  (`self.GetAxisSpawnData`)
  (`self.InitFoodIDMetaData`))