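; BP_LeftHand is the VR left hand that carries a filter menu, toggled when a BP_Hand overlaps its box.
; OpenMenu spawns BP_FilterMenu attached at FilterPlace and CloseMenu destroys it, with InMenu tracking state.
; IsMenuDetached blocks toggling; DetachMenu sets it and ReturnToOwner clears it, unhides the UI and destroys the menu.
; Pickup and Drop are empty, their detach logic unwired, and DetachMenu clears ChildMenu before returning it.
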(event `self.ReceiveBeginPlay`
  (`parent.ReceiveBeginPlay`))

(event `self.Box_0.OnComponentBeginOverlap`
  (params (OverlappedComponent :type "PrimitiveComponent Object Reference") (OtherActor :type "Actor Object Reference") (OtherComp :type "PrimitiveComponent Object Reference") (OtherBodyIndex :type Integer) (bFromSweep :type Boolean) (SweepResult :type "HitResult Structure (by ref)"))
  (cast `/Game/Blueprints/VR_Character/BP_Hand` OtherActor)
  (if (not (`self.IsMenuDetached`))
    (if (`self.InMenu`)
      (`self.CloseMenu`)
      (else
        (`self.OpenMenu`)))))

(event `/Game/Blueprints/Util/BPI_Interactions.Pickup`
  (params (AttachTo :type "SceneComponent Object Reference")))

(event `/Game/Blueprints/Util/BPI_Interactions.Drop`)

(fn `CloseMenu`
  (`self.K2_DestroyActor` (`self.ChildMenu`))
  (set `self.InMenu` false))

(fn `DetachMenu`
  (returns (Child :type "/Game/Blueprints/VR_Character/BP_FilterMenu Object Reference"))
  (`SceneComponent.K2_DetachFromComponent` (`self.FilterPlace`) "KeepWorld" "KeepRelative" "KeepWorld" true)
  (bind _output_get (set `self.ChildMenu` null))
  (set `self.IsMenuDetached` true)
  (return _output_get))

(fn `HideMenu`
  (params (Hide :type Boolean))
  (`/Game/Blueprints/VR_Character/WBP_Inventory.hide` (`self.UI`) Hide))

(fn `OpenMenu`
  (bind _returnvalue (`|SpawnActorFromClass` "/Game/Blueprints/VR_Character/BP_FilterMenu.BP_FilterMenu_C" (`SceneComponent.K2_GetComponentToWorld` (`self.FilterPlace`)) "AlwaysSpawn" "OverrideRootScale" null self null))
  (set `self.ChildMenu` _returnvalue)
  (`self.K2_AttachToComponent` _returnvalue (`self.FilterPlace`) "None" "KeepWorld" "KeepWorld" "KeepWorld" false)
  (set `self.InMenu` true))

(fn `ReturnToOwner`
  (`self.HideMenu` false)
  (set `self.IsMenuDetached` false)
  (`self.K2_DestroyActor` (`self.ChildMenu`))
  (return))

(fn `ToggleMenuStay`)

(fn `UserConstructionScript`
  (`parent.UserConstructionScript`))