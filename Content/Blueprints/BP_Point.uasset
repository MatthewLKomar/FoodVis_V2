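; BP_Point is a point Actor that BP_MotionController can pick up and drop.
; Pickup attaches its root component to the given component and Drop detaches it, both keeping the world transform.
; The construction script applies a configurable sprite to its Billboard, and BeginPlay records the starting location.
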(event `/Game/Blueprints/Util/BPI_Interactions.Pickup`
  (params (AttachTo :type "SceneComponent Object Reference"))
  (`SceneComponent.K2_AttachToComponent` (`self.K2_GetRootComponent`) AttachTo "None" "KeepWorld" "KeepWorld" "KeepWorld" false))

(event `self.ReceiveBeginPlay`
  (set `self.StartLocation` (`self.K2_GetActorLocation`)))

(event `/Game/Blueprints/Util/BPI_Interactions.Drop`
  (`self.K2_DetachFromActor` "KeepWorld" "KeepWorld" "KeepWorld"))

(fn `UserConstructionScript`
  (`BillboardComponent.SetSprite` (`self.Billboard`) (`self.SpriteUsed`)))