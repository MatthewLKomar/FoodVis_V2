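; BP_Axis is a labeled vertical axis actor that plots food entries from a data table as points at heights mapped from their normalized values.
; Construction fills a map of food IDs to coordinates and entries, placing foods missing from the table at zero value.
; BeginPlay spawns and attaches a BP_Point for each, caching pivot-relative offsets.
; ScaleVertical repositions points from those offsets to stretch the axis without cumulative scaling.
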(event `self.ReceiveBeginPlay`
  (`TextRenderComponent.K2_SetText` (`self.TextRender`) (`self.Name`))
  (`self.Spawn Data Points`))

(fn `CreateNullPoints`
  (params (Food_IDs :type "Array of Integer"))
  (bind (_returnvalue_x _returnvalue_y _returnvalue_z) (`KismetMathLibrary.BreakVector` (`self.K2_GetActorLocation`)))
  (bind _pointcoords (`self.PointCoords`))
  (for _array_element Food_IDs
    (if (not (`.ReturnValue` (`BlueprintMapLibrary.Map_Find` _pointcoords _array_element)))
      (`BlueprintMapLibrary.Map_Add` _pointcoords _array_element (make `/Game/FlavorData/FPoint` (`KismetMathLibrary.MakeVector` _returnvalue_x _returnvalue_y (+ _returnvalue_z (`self.GeneratePointHeight` 0.0))))))))

(fn `CreatePoints`
  (locals (FoodID_holder :type Integer))
  (bind (_returnvalue_x _returnvalue_y _returnvalue_z) (`KismetMathLibrary.BreakVector` (`self.K2_GetActorLocation`)))
  (bind (_returnvalue_x_2 _returnvalue_y_2 _returnvalue_z_2) (`KismetMathLibrary.BreakVector` (`self.K2_GetActorLocation`)))
  (bind _food_ids (`/Game/Blueprints/Util/BP_FoodVis_Funcs.GetFood_IDs`))
  (for _array_element _food_ids
    (bind _output_get (set `local.FoodID_holder` _array_element))
    ;[1 1 1] try to find food id in current data
    (bind (_found_ _entry) (`self.FindFoodinDT` _output_get))
    (if _found_
      (bind (_source_id _food_id _flavor_name _food_name _orig_content _flavor_group _normalized) (break `/Game/FlavorData/FEntry` _entry))
      (`BlueprintMapLibrary.Map_Add` (`self.PointCoords`) _food_id (make `/Game/FlavorData/FPoint` (`KismetMathLibrary.MakeVector` _returnvalue_x _returnvalue_y (+ _returnvalue_z (`self.GeneratePointHeight` _normalized))) _entry))
      (else
        ;[1 1 1] didn't find the food, create dummy 0 node
        (`BlueprintMapLibrary.Map_Add` (`self.PointCoords`) (`local.FoodID_holder`) (make `/Game/FlavorData/FPoint` (`KismetMathLibrary.MakeVector` _returnvalue_x_2 _returnvalue_y_2 (+ _returnvalue_z_2 (`self.GeneratePointHeight` 0.0)))))))))

(fn `FindFoodIDHelper`
  (params (ID :type Integer))
  (returns (Found :type Boolean) (`Array Index` :type Integer))
  (locals (indexFound :type Integer :default -1) (`Found?` :type Boolean))
  (bind _returnvalue (`DataTableFunctionLibrary.GetDataTableColumnAsString` (`self.DataTable`) "food_id"))
  (bind _returnvalue_2 (`KismetArrayLibrary.Array_Find` _returnvalue (`KismetStringLibrary.Conv_IntToString` ID)))
  (if (!= _returnvalue_2 -1)
    (set `local.indexFound` _returnvalue_2)
    (set `local.Found?` true)
    (return (`local.Found?`) (`local.indexFound`))
    (else
      (return (`local.Found?`) (`local.indexFound`)))))

(fn `FindFoodinDT`
  (params (FoodID :type Integer))
  (returns (`Found?` :type Boolean) (Entry :type "/Game/FlavorData/FEntry Structure"))
  (bind (_found _array_index) (`self.FindFoodIDHelper` FoodID))
  (bind _datatable (`self.DataTable`))
  ;[1 1 1] not found
  (if _found
    (bind _outrownames (`DataTableFunctionLibrary.GetDataTableRowNames` _datatable))
    (bind _returnvalue (`|GetDataTableRow` _datatable (`|GetArrayItem` _outrownames _array_index))
      (:`then`
        ;[1 1 1] found, return true and the entry
        (return true _returnvalue))
      (:`RowNotFound`
        (`KismetSystemLibrary.PrintString` "FINDFoodID,BPAXIS, shouldn't have happened")))
    (else
      ;[1 1 1] not found, return false
      (return false))))

(fn `GeneratePointHeight`
  (params (Value :type "Float (double-precision)"))
  (returns (ReturnValue :type "Float (double-precision)"))
  (return (`KismetMathLibrary.MapRangeClamped` Value 0.0 1.0 (`self.MinHeight`) (`self.Height`))))

(fn `ScaleVertical`
  (params (Scale :type "Float (double-precision)"))
  (for (_array_element _array_index) (`self.PointReferences`)
    (bind (_output_x _output_y _output_z) (`KismetMathLibrary.BreakVector` (`|GetArrayItem` (`self.OrigLocation`) _array_index)))
    (`self.K2_SetActorLocation` _array_element (+ (`KismetMathLibrary.MakeVector` _output_x _output_y (* Scale _output_z)) (`self.PointsPivot`)) false false)))

(fn `Spawn Data Points`
  (bind _pointcoords (`self.PointCoords`))
  (bind _keys (`BlueprintMapLibrary.Map_Keys` _pointcoords))
  (for _array_element _keys
    (bind _value (`BlueprintMapLibrary.Map_Find` _pointcoords _array_element))
    (`KismetArrayLibrary.Array_Add` (`self.OrigLocation`) (- (break `/Game/FlavorData/FPoint` _value) (`self.PointsPivot`)))
    (bind _returnvalue (`|SpawnActorFromClass` "/Game/Blueprints/BP_Point.BP_Point_C" (`KismetMathLibrary.MakeTransform` (break `/Game/FlavorData/FPoint` _value)) "Undefined" "OverrideRootScale" null (`.Food_ID_4_8622C12A4BFD36B656F6D3868216950A` (break `/Game/FlavorData/FPoint` _value)) null))
    (`self.K2_AttachToActor` _returnvalue self "None" "KeepWorld" "KeepWorld" "KeepWorld" true)
    (`KismetArrayLibrary.Array_Add` (`self.PointReferences`) _returnvalue)))

(fn `UserConstructionScript`
  (locals (All_Food_IDs :type "Array of Integer"))
  (bind _food_ids (`/Game/Blueprints/Util/BP_FoodVis_Funcs.GetFood_IDs`))
  (set `local.All_Food_IDs` _food_ids)
  (`self.CreatePoints`)
  ;[1 1 1] includes offset for the cube
  (set `self.PointsPivot` (+ (`SceneComponent.K2_GetComponentLocation` (`self.DefaultSceneRoot`)) (0.0 0.0 50.0))))