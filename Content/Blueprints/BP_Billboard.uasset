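; BP_Billboard is a billboard actor that a motion controller can pick up and drop.
; On BeginPlay, flag A selects one of two stored placements and teleports the actor there.
; The A branch also applies a cauliflower material to Descriptor and offsets the height and yaw.
; Pickup attaches the root to the supplied component and Drop detaches it, both keeping the world transform.
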(event `self.ReceiveBeginPlay`
  (bind (_rotb_x _rotb_y _rotb_z) (`KismetMathLibrary.BreakVector` (`self.RotB`)))
  (bind (_rota_x _rota_y _rota_z) (`KismetMathLibrary.BreakVector` (`self.RotA`)))
  (if (`self.A`)
    (`PrimitiveComponent.SetMaterial` (`self.Descriptor`) 0 "/Game/Assets/Billboards/M_Cauliflower.M_Cauliflower")
    (`self.K2_SetActorRotation` (`KismetMathLibrary.MakeRotator` 0.0 0.0 (+ _rota_z -90.0)))
    (`self.K2_SetActorLocation` (+ (`self.VecA`) (0.0 0.0 100.0)) false true)
    (else
      (`self.K2_SetActorRotation` (`KismetMathLibrary.MakeRotator` 0.0 0.0 _rotb_z))
      (`self.K2_SetActorLocation` (`self.VecB`) false true))))

(event `/Game/Blueprints/Util/BPI_Interactions.Pickup`
  (params (AttachTo :type "SceneComponent Object Reference"))
  (`SceneComponent.K2_AttachToComponent` (`self.K2_GetRootComponent`) AttachTo "None" "KeepWorld" "KeepWorld" "KeepWorld" false))

(event `/Game/Blueprints/Util/BPI_Interactions.Drop`
  (`self.K2_DetachFromActor` "KeepWorld" "KeepWorld" "KeepWorld"))

(fn `UserConstructionScript`)